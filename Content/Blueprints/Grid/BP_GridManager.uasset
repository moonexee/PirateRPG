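; Grid manager that builds the tile board and places the starting units for a turn-based, grid-based game.
; After a short delay on BeginPlay, it spawns BP_Tile actors with random movement costs and registers each cell in BP_MyPathfinder's Grid.
; It spawns three enemies and three players on preset cells, recording each as the cell's Occupier.
; BP_TurnManager then stores the units, and the pathfinder initializes the grid.
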(event `self.ReceiveBeginPlay`
  (bind _returnvalue (`GameplayStatics.GetActorOfClass` "/Game/Blueprints/BP_MyPathfinder.BP_MyPathfinder_C"))
  (bind _output_get (set `self.Ref_Pathfinder` _returnvalue))
  (`KismetSystemLibrary.Delay` 0.2)
  (`self.GenerateGrid`)
  (`Pathfinder.InitializeGrid` _output_get))

(event `GenerateGrid`
  (bind _returnvalue (+ (`self.TileSize`) (`self.TileSpacing`)))
  ;[0.4941 1 0.6784] X-grid
  (for _index (range (`self.GridHeight`))
    ;[1 0.5608 0.5608] Y-grid
    (for _index_2 (range (`self.GridWidth`))
      (bind _result (`/Engine/EditorBlueprintResources/StandardMacros.IncrementInt` (`self.CellID`))
        (:`  `
          (bind _output_get (set `self.CellID` _result))
          (bind _returnvalue_2 (`KismetMathLibrary.MakeVector` (* _index _returnvalue) (* _index_2 _returnvalue) 2.0))
          (bind _returnvalue_3 (`|SpawnActorFromClass` "/Game/Blueprints/Grid/BP_Tile.BP_Tile_C" (`KismetMathLibrary.MakeTransform` _returnvalue_2) "Undefined" "MultiplyWithRoot" null (`KismetMathLibrary.RandomIntegerInRange` 1 2) _output_get null))
          ;[1 1 1] add the spawned tiles into an array
          (`KismetArrayLibrary.Array_Add` (`self.GridArray`) _returnvalue_3)
          (`KismetArrayLibrary.Array_AddUnique` (`Pathfinder.Grid` (`self.Ref_Pathfinder`)) (make `GridCell` _output_get _returnvalue_2 (`/Game/Blueprints/Grid/BP_Tile.Cost` _returnvalue_3)))))))
  ;[1 0.8758 0.6159] Spawn in the Enemies and Players on specific tiles
  (for _ (range 3)
    (`self.SpawnEnemies` (`|GetArrayItem` (`self.EnemiesSpawn`) (`self.PlacementIndex`))))
  (set `self.PlacementIndex` 0)
  (for _ (range 3)
    (`self.SpawnPlayers` (`|GetArrayItem` (`self.PlayerSpawn`) (`self.PlacementIndex`))))
  ;[1 1 1] Sets the Spawned in Units in the Turn Manager
  (bind _returnvalue_4 (`GameplayStatics.GetActorOfClass` "/Game/Blueprints/BP_TurnManager.BP_TurnManager_C"))
  (`/Game/Blueprints/BP_TurnManager.Store Units` _returnvalue_4))

(fn `SpawnEnemies`
  (params (CellID :type Integer))
  (bind (_output_id _output_gridposition _output_cost _output_linkedcells) (break `GridCell` (`|GetArrayItem` (`Pathfinder.Grid` (`self.Ref_Pathfinder`)) CellID)))
  ;[0 0 0] Spawns Enemies and sets the Grid data then increases the placement index
  (if (< (`self.PlacementIndex`) 3)
    (bind _asbp_unit_base_enemies (castclass `/Game/Blueprints/Units/Enemies/BP_UnitBase_Enemies` (`|GetArrayItem` (`self.Enemies`) (`self.PlacementIndex`))))
    (bind _returnvalue (`|SpawnActorFromClass` _asbp_unit_base_enemies (`KismetMathLibrary.MakeTransform` _output_gridposition (struct :`Yaw` 180.0)) "Undefined" "MultiplyWithRoot" null _output_id null))
    (`KismetArrayLibrary.Array_Set` (`Pathfinder.Grid` (`self.Ref_Pathfinder`)) CellID (make `GridCell` _output_id _output_gridposition _output_cost _output_linkedcells _returnvalue))
    (`/Engine/EditorBlueprintResources/StandardMacros.IncrementInt` (`self.PlacementIndex`))))

(fn `SpawnPlayers`
  (params (CellID :type Integer))
  (bind (_output_id _output_gridposition _output_cost _output_linkedcells) (break `GridCell` (`|GetArrayItem` (`Pathfinder.Grid` (`self.Ref_Pathfinder`)) CellID)))
  ;[0 0 0] Spawns Players and sets the Grid data then increases the placement index
  (if (< (`self.PlacementIndex`) 3)
    (bind _asbp_unit_base_player (castclass `/Game/Blueprints/Units/Players/BP_UnitBase_Player` (`|GetArrayItem` (`self.Players`) (`self.PlacementIndex`))))
    (bind _returnvalue (`|SpawnActorFromClass` _asbp_unit_base_player (`KismetMathLibrary.MakeTransform` _output_gridposition) "Undefined" "MultiplyWithRoot" null _output_id null))
    (`KismetArrayLibrary.Array_Set` (`Pathfinder.Grid` (`self.Ref_Pathfinder`)) CellID (make `GridCell` _output_id _output_gridposition _output_cost _output_linkedcells _returnvalue))
    (`/Engine/EditorBlueprintResources/StandardMacros.IncrementInt` (`self.PlacementIndex`))))

(fn `UserConstructionScript`)