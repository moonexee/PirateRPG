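; BP_Tile is a clickable grid tile for turn-based tactics, shaded by its movement cost.
; At BeginPlay it finds the grid and turn managers.
; On a click during the player's turn it checks the move or fight mode in the actions widget, then asks the current unit to validate the tile and move or attack there.
; HighlightRange and ResetColor swap materials to show or clear ranges.
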(event `self.ReceiveBeginPlay`
  (bind _returnvalue (`GameplayStatics.GetActorOfClass` "/Game/Blueprints/Grid/BP_GridManager.BP_GridManager_C"))
  (set `self.Ref_GridManager` _returnvalue)
  (bind _returnvalue_2 (`GameplayStatics.GetActorOfClass` "/Game/Blueprints/BP_TurnManager.BP_TurnManager_C"))
  (set `self.Ref_TurnManager` _returnvalue_2)
  (if (> (`self.Cost`) 1)
    (`PrimitiveComponent.SetMaterial` (`self.StaticMesh`) 0 (`self.M_Cost`))
    (else
      (`PrimitiveComponent.SetMaterial` (`self.StaticMesh`) 0 (`self.M_Default`)))))

(event `self.ReceiveActorOnClicked`
  (params (ButtonPressed :type "Key Structure"))
  (if (`/Game/Blueprints/BP_TurnManager.isPlayerTurn` (`self.Ref_TurnManager`))
    (`self.ClickTile`)))

(event `ClickTile`
  (bind _wbp_actions (`/Game/Blueprints/BP_TurnManager.WBP_Actions` (`self.Ref_TurnManager`)))
  (bind _currentunit (`/Game/Blueprints/BP_TurnManager.CurrentUnit` (`self.Ref_TurnManager`)))
  ;[1 0.505 0.5749] Clicked
  (`/Engine/EditorBlueprintResources/StandardMacros.IsValid` _wbp_actions
    (:`Is Valid`
      (if (`/Game/UI/WBP_Actions.isMoveClicked` _wbp_actions)
        (bind _returnvaluemove (`/Game/Blueprints/Units/BP_UnitBase.IsCellClickable(Move)?` (`/Game/Blueprints/BP_TurnManager.CurrentUnit` (`self.Ref_TurnManager`)) (`self.IDTile`)))
        (if _returnvaluemove
          (`PrimitiveComponent.SetMaterial` (`self.StaticMesh`) 0 (`self.M_Select`))
          (set `/Game/Blueprints/Grid/BP_GridManager.SelectedTile` self (`self.Ref_GridManager`))
          (`/Game/Blueprints/Units/BP_UnitBase.MoveToDestination` (`/Game/Blueprints/BP_TurnManager.CurrentUnit` (`self.Ref_TurnManager`)) (`self.IDTile`)))
        (elif (`/Game/UI/WBP_Actions.isFightClicked` _wbp_actions)
          (bind _newparam (`/Game/Blueprints/Units/BP_UnitBase.IsCellClickable(Attack)?` (`/Game/Blueprints/BP_TurnManager.CurrentUnit` (`self.Ref_TurnManager`)) (`self.IDTile`)))
          (if _newparam
            (`PrimitiveComponent.SetMaterial` (`self.StaticMesh`) 0 (`self.M_Action`))
            (if (`KismetSystemLibrary.IsValid` _currentunit)
              (`CUnitBase.PerformAttack` _currentunit (`CUnitBase.CurrentAttackType` _currentunit) (`self.IDTile`)))))))))

(fn `HighlightRange`
  (params (Active :type Boolean))
  (if Active
    (`PrimitiveComponent.SetMaterial` (`self.StaticMesh`) 0 (`self.M_Action`))
    (else
      (`self.ResetColor`))))

(fn `ResetColor`
  (if (> (`self.Cost`) 1)
    (`PrimitiveComponent.SetMaterial` (`self.StaticMesh`) 0 (`self.M_Cost`))
    (else
      (`PrimitiveComponent.SetMaterial` (`self.StaticMesh`) 0 (`self.M_Default`)))))

(fn `UserConstructionScript`)