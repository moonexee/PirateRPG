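; Base enemy unit for the grid-based, turn-based combat that makes the AI's decision to attack or move.
; MakeDecision collects player units in range through the pathfinder, using adjacent cells for BP_UnitBase_E2 and AttackRange for other enemies.
; FinalDecision attacks the first target found, otherwise moves to a random linked cell of the nearest player.
; If that cell is occupied, FinalDecision calls itself again to re-roll.
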(event `self.ReceiveBeginPlay`
  (`parent.ReceiveBeginPlay`))

(event `self.MakeDecision`
  (bind (_unitstats_maxhealth _unitstats_health _unitstats_level _unitstats_xp _unitstats_attack _unitstats_attackrange) (break `UnitStats` (`self.UnitStats`)))
  (bind _currentunit (`/Game/Blueprints/BP_TurnManager.CurrentUnit` (`self.Ref_TurnManager`)))
  (for _array_element (`/Game/Blueprints/BP_TurnManager.PlayerUnits` (`self.Ref_TurnManager`))
    (if (== (`GameplayStatics.GetObjectClass` _currentunit) "/Game/Blueprints/Units/Enemies/BP_UnitBase_E2.BP_UnitBase_E2_C")
      (bind _returnvalue (`Pathfinder.GetAdjacentCells` (`self.Ref_Pathfinder`) (`CUnitBase.CurrentID` _currentunit)))
      (bind _currentid (`CUnitBase.CurrentID` _array_element))
      (if (`KismetArrayLibrary.Array_Contains` _returnvalue _currentid)
        (`KismetArrayLibrary.Array_AddUnique` (`self.Players`) _currentid))
      (else
        (bind _returnvalue_2 (`Pathfinder.GetReachableCells` (`self.Ref_Pathfinder`) (`CUnitBase.CurrentID` (`/Game/Blueprints/BP_TurnManager.CurrentUnit` (`self.Ref_TurnManager`))) _unitstats_attackrange))
        (if (`KismetArrayLibrary.Array_Contains` _returnvalue_2 _currentid)
          (`KismetArrayLibrary.Array_AddUnique` (`self.Players`) _currentid)))))
  (`self.FinalDecision`))

(event `FinalDecision`
  (bind _players (`self.Players`))
  (if (`KismetArrayLibrary.Array_IsEmpty` _players)
    (set `self.ClosestDistance` 999999.0)
    (set `self.TargetPlayerID` 0)
    (bind (_closestid _returnvalue) (`self.GetClosestID`))
    (if _returnvalue
      (`self.FinalDecision`)
      (else
        (`self.Move` _closestid)))
    (else
      (`self.PerformAttack` (`CUnitBase.CurrentAttackType` (`/Game/Blueprints/BP_TurnManager.CurrentUnit` (`self.Ref_TurnManager`))) (`|GetArrayItem` _players))
      (`KismetArrayLibrary.Array_Clear` (`self.Players`)))))

(fn `GetClosestID`
  (returns (ClosestID :type Integer) (ReturnValue :type Boolean))
  (bind _grid (`Pathfinder.Grid` (`self.Ref_Pathfinder`)))
  (bind (_output_id _output_gridposition _output_cost _output_linkedcells) (break `GridCell` (`|GetArrayItem` (`Pathfinder.Grid` (`self.Ref_Pathfinder`)) (`self.PlayerID`))))
  (bind (_output_id_2 _output_gridposition_2) (break `GridCell` (`|GetArrayItem` (`Pathfinder.Grid` (`self.Ref_Pathfinder`)) (`self.EnemyID`))))
  (bind _returnvalue (`KismetMathLibrary.Vector_Distance` _output_gridposition _output_gridposition_2))
  (bind _output_id_3 (break `GridCell` (`|GetArrayItem` _grid (`KismetArrayLibrary.Array_Random` _output_linkedcells))))
  ;[1 0.5747 0.4542] Gets Player IDs and Enemy IDs
  (for _array_element (`/Game/Blueprints/BP_TurnManager.PlayerUnits` (`self.Ref_TurnManager`))
    (set `self.PlayerID` (`CUnitBase.CurrentID` _array_element))
    (set `self.EnemyID` (`self.CurrentID`))
    (if (< _returnvalue (`self.ClosestDistance`))
      (set `self.ClosestDistance` _returnvalue)
      (bind _output_get (set `self.TargetPlayerID` _output_id_3))))
  (bind (_output_id_4 _output_gridposition_3 _output_cost_2 _output_linkedcells_2 _output_occupier) (break `GridCell` (`|GetArrayItem` _grid _output_get)))
  (return _output_get (`KismetSystemLibrary.IsValid` _output_occupier)))

(fn `UserConstructionScript`
  (`parent.UserConstructionScript`))